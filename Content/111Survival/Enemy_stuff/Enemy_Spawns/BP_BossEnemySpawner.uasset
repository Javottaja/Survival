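; Boss enemy spawner that spawns a random AI pawn from its enemy list late in the survival round.
; On Tick it waits for the Playing state with spawning enabled in BP_StoreVars on the game instance, then DoOnce starts a delay of 80% of WinTime.
; It then spawns at a fixed offset from the actor found for a randomly picked spawn-point class.
; An author note flags the Tick polling for replacement by a timer.
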(event `self.ReceiveTick`
  (params (DeltaSeconds :type "Float (single-precision)"))
  ;[1 1 1] DO NOT TICK THIS, use timer or sumthin
  ;;[1 1 1] Read GameState and act accordingly
  (bind _asbp_store_vars (cast `/Game/111Survival/BP_StoreVars` (`GameplayStatics.GetGameInstance`)))
  (switch `/Game/111Survival/EN_GameState` (`/Game/111Survival/BP_StoreVars.GameState` _asbp_store_vars)
    (:`NewEnumerator1`
      ;;[1 1 1] Loop as long as Spawn New Enemies = true
      (if (`/Game/111Survival/BP_StoreVars.bSpawnNewEnemies` _asbp_store_vars)
        (`/Engine/EditorBlueprintResources/StandardMacros.DoOnce` false
          (:`Completed`
            (bind _delay (`self.CalculateSpawnDelay` _asbp_store_vars))
            (`KismetSystemLibrary.Delay` _delay)
            ;[1 1 1] Get random location for spawning
            (bind _returnvalue (`GameplayStatics.GetActorOfClass` (`|GetArrayItem` (`self.EnemySpawnPoints`) (`KismetMathLibrary.RandomIntegerInRange` 0 (- (`KismetArrayLibrary.Array_Length` (`self.EnemySpawnPoints`)) 1)))))
            (`AIBlueprintHelperLibrary.SpawnAIFromClass` (`|GetArrayItem` (`self.EnemiesToSpawn`) (`KismetMathLibrary.RandomIntegerInRange` 0 (- (`KismetArrayLibrary.Array_Length` (`self.EnemiesToSpawn`)) 1))) null (- (`self.K2_GetActorLocation` _returnvalue) (400.0 100.0 -300.0)) (`self.K2_GetActorRotation` _returnvalue) true null)))))))

(fn `CalculateSpawnDelay`
  (params (StoreVarsRef :type "/Game/111Survival/BP_StoreVars Object Reference"))
  (returns (Delay :type "Float (double-precision)"))
  (return (* (`/Game/111Survival/BP_StoreVars.WinTime` StoreVarsRef) 0.8)))

(fn `UserConstructionScript`)