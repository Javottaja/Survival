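; Basic enemy spawner that spawns random enemy pawns at random spawn points while the game state is Playing.
; Tick drives a Delay-paced loop, gated by the BP_StoreVars game instance's spawn flag and a cap on its debug alive-enemy counter, which each spawn increments.
; CalculateSpawnDelay scales the interval with remaining round time, clamped between fastest and slowest settings, so spawns speed up as the round progresses.
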(event `self.ReceiveTick`
  (params (DeltaSeconds :type "Float (single-precision)"))
  ;[1 1 1] Read GameState and act accordingly
  (bind _asbp_store_vars (cast `/Game/111Survival/BP_StoreVars` (`GameplayStatics.GetGameInstance`)))
  (switch `/Game/111Survival/EN_GameState` (`/Game/111Survival/BP_StoreVars.GameState` _asbp_store_vars)
    (:`NewEnumerator1`
      ;[1 1 1] Loop as long as Spawn New Enemies = true
      (if (and (`/Game/111Survival/BP_StoreVars.bSpawnNewEnemies` _asbp_store_vars) (< (`/Game/111Survival/BP_StoreVars.DEBUG_AliveBasicEnemies` _asbp_store_vars) 300))
        (bind _delay (`self.CalculateSpawnDelay` _asbp_store_vars))
        (`KismetSystemLibrary.Delay` _delay)
        ;[1 1 1] Get random location for spawning
        (bind _returnvalue (`GameplayStatics.GetActorOfClass` (`|GetArrayItem` (`self.EnemySpawnPoints`) (`KismetMathLibrary.RandomIntegerInRange` 0 (- (`KismetArrayLibrary.Array_Length` (`self.EnemySpawnPoints`)) 1)))))
        (`AIBlueprintHelperLibrary.SpawnAIFromClass` (`|GetArrayItem` (`self.EnemiesToSpawn`) (`KismetMathLibrary.RandomIntegerInRange` 0 (- (`KismetArrayLibrary.Array_Length` (`self.EnemiesToSpawn`)) 1))) null (`self.K2_GetActorLocation` _returnvalue) (`self.K2_GetActorRotation` _returnvalue) false null)
        ;[1 1 1] Increment Alive Enemies counter
        (bind _asbp_store_vars_2 (cast `/Game/111Survival/BP_StoreVars` (`GameplayStatics.GetGameInstance`)))
        (`/Engine/EditorBlueprintResources/StandardMacros.IncrementInt` (`/Game/111Survival/BP_StoreVars.DEBUG_AliveBasicEnemies` _asbp_store_vars_2))))))

(fn `CalculateSpawnDelay`
  (params (StoreVarsRef :type "/Game/111Survival/BP_StoreVars Object Reference"))
  (returns (Delay :type "Float (double-precision)"))
  (bind _enemyspawnfreqslowest (`/Game/111Survival/BP_StoreVars.EnemySpawnFreqSlowest` StoreVarsRef))
  (bind _enemyspawnfreqfastest (`/Game/111Survival/BP_StoreVars.EnemySpawnFreqFastest` StoreVarsRef))
  (return (`KismetMathLibrary.FClamp` (- (* (/ (- _enemyspawnfreqslowest _enemyspawnfreqfastest) 100.0) (* (/ (`/Game/111Survival/BP_StoreVars.RoundTimeLeft` StoreVarsRef) (`/Game/111Survival/BP_StoreVars.WinTime` StoreVarsRef)) 100.0)) _enemyspawnfreqfastest) _enemyspawnfreqfastest _enemyspawnfreqslowest)))

(fn `UserConstructionScript`)