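; BP_ToughEnemy_Basic is an enemy Blueprint that fires at the player when close and in plain view.
; A looping half-second timer, started on BeginPlay, line-traces on the Visibility channel from the enemy to the player.
; When the trace hits a BP_PlayerCharacter within range, it passes the look-at direction to FireShot, which is defined outside this graph.
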(event `self.ReceiveBeginPlay`
  (`KismetSystemLibrary.K2_SetTimer` null "GetDistanceToPlayer" 0.5 true))

(event `GetDistanceToPlayer`
  ;[1 1 1] Get distance to player
  (bind _outhit (`KismetSystemLibrary.LineTraceSingle` :`Start` (`self.K2_GetActorLocation`) :`End` (`self.K2_GetActorLocation` (`GameplayStatics.GetPlayerCharacter` 0)) :`TraceChannel` "TraceTypeQuery1" :`TraceColor` (struct :`R` 0.117121 :`B` 1.0 :`A` 1.0) :`DrawTime` 0.5))
  ;[1 1 1] Check conditions for firing
  (`/Engine/EditorBlueprintResources/StandardMacros.IsValid` (`.HitActor` (`GameplayStatics.BreakHitResult` _outhit))
    (:`Is Valid`
      (if (and (<= (`.Distance` (`GameplayStatics.BreakHitResult` _outhit)) 600.0) (`KismetMathLibrary.ClassIsChildOf` (`GameplayStatics.GetObjectClass` (`.HitActor` (`GameplayStatics.BreakHitResult` _outhit))) "/Game/111Survival/BP_PlayerCharacter.BP_PlayerCharacter_C"))
        ;[1 1 1] Rotate and shoot
        (`self.FireShot` (`KismetMathLibrary.Conv_RotatorToVector` (`KismetMathLibrary.FindLookAtRotation` (`self.K2_GetActorLocation`) (`self.K2_GetActorLocation` (`.HitActor` (`GameplayStatics.BreakHitResult` _outhit))))))))))

(fn `UserConstructionScript`
  (`parent.UserConstructionScript`))