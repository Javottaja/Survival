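; First boss enemy for the 111Survival mode, a child Blueprint that adds a timed attack and a cinematic entrance.
; On BeginPlay a looping timer starts, periodically calling FireShot at the boss's location.
; If a spawn sound is set, it plays while MousePlayerController focuses the camera on the boss in slow motion, then switches target and restores normal speed.
; A note says this intro belongs in the parent class.
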(event `self.ReceiveBeginPlay`
  (`KismetSystemLibrary.K2_SetTimerDelegate` (delegate `FirePulse`) 7.0 true)
  (bind _spawnsound (`self.SpawnSound`)
    (:`then`
      (`GameplayStatics.PlaySound2D` _spawnsound 1.0 1.0 0.0 null null)
      ;[1 1 1] Wrong place, this should be done in parent
      (bind _asmouse_player_controller (cast `/Game/111Survival/MousePlayerController` (`GameplayStatics.GetPlayerController` 0)))
      (`/Game/111Survival/MousePlayerController.FocusCameraOnBoss` _asmouse_player_controller self)
      (`GameplayStatics.SetGlobalTimeDilation` 0.2)
      (`KismetSystemLibrary.Delay` 0.4)
      (`/Game/111Survival/MousePlayerController.ChangeCameraTarget` _asmouse_player_controller null)
      (`GameplayStatics.SetGlobalTimeDilation` 1.0))
    (:`else`)))

(event `FirePulse`
  (`self.FireShot` (`self.K2_GetActorLocation`)))

(fn `UserConstructionScript`
  (`parent.UserConstructionScript`))