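; Base boss enemy Blueprint that extends an enemy parent class with boss health bar display.
; On construction it fetches the boss stats reference from the BP_StoreVars game instance, registers itself and shows the stats.
; Any damage runs parent logic, then refreshes the health bar.
; DestroyEnemy hides the stats and plays a death sound, calling parent destruction only when both stats reference and sound are valid.
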(event `self.ReceiveAnyDamage`
  (params (Damage :type "Float (single-precision)") (DamageType :type "DamageType Object Reference") (InstigatedBy :type "Controller Object Reference") (DamageCauser :type "Actor Object Reference"))
  (`parent.ReceiveAnyDamage` Damage null null null)
  (`self.UpdatePlayerWidgetReference`))

(fn `DestroyEnemy`
  (bind _bossstatsref (`self.BossStatsRef`)
    (:`then`
      (`/Game/111Survival/UI/UI_BossStats.HideBossStats` _bossstatsref)
      (bind _deathsound (`self.DeathSound`)
        (:`then`
          (`GameplayStatics.PlaySound2D` _deathsound 1.0 1.0 0.0 null null)
          (`parent.DestroyEnemy`))
        (:`else`)))
    (:`else`)))

(fn `UpdatePlayerWidgetReference`
  (bind _bossstatsref (`self.BossStatsRef`)
    (:`then`
      (set `/Game/111Survival/UI/UI_BossStats.BossReference` self _bossstatsref)
      (`/Game/111Survival/UI/UI_BossStats.UpdateBossHealthBar` _bossstatsref))
    (:`else`
      (`KismetSystemLibrary.PrintString` "Couldn't set Boss reference!" true true (struct :`R` 1.0 :`B` 0.10674 :`A` 1.0) 5.0))))

(fn `UserConstructionScript`
  (`parent.UserConstructionScript`)
  (bind _asbp_store_vars (cast `/Game/111Survival/BP_StoreVars` (`GameplayStatics.GetGameInstance`)))
  (set `self.BossStatsRef` (`/Game/111Survival/BP_StoreVars.BossStatsRef` _asbp_store_vars))
  (`self.UpdatePlayerWidgetReference`)
  (bind _bossstatsref (`self.BossStatsRef`)
    (:`then`
      (`/Game/111Survival/UI/UI_BossStats.ShowBossStats` _bossstatsref))
    (:`else`)))