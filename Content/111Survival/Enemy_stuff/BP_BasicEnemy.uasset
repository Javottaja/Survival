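; BP_BasicEnemy is a basic enemy with health that deals contact damage in the game.
; Incoming damage lowers current health, and at zero it destroys the capsule, mesh and actor.
; On hit, it damages actors that implement BPI_Damageable and carry the "Friend" tag.
; An unconnected branch would spawn an explosion effect stored as FireExplosion, whose EndPlay event is set to destroy the enemy.
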(event `self.ReceiveAnyDamage`
  (params (Damage :type "Float (single-precision)") (DamageType :type "DamageType Object Reference") (InstigatedBy :type "Controller Object Reference") (DamageCauser :type "Actor Object Reference"))
  ;[1 1 1] Take damage, and if health drops to 0, destroy enemy
  (bind _output_get (set `self.HealthCurrent` (- (`self.HealthCurrent`) Damage)))
  (if (<= _output_get 0.0)
    (`ActorComponent.K2_DestroyComponent` (`self.CapsuleComponent`))
    (`ActorComponent.K2_DestroyComponent` (`self.Mesh`))
    (`self.K2_DestroyActor`)))

(event `self.ReceiveHit`
  (params (MyComp :type "PrimitiveComponent Object Reference") (Other :type "Actor Object Reference") (OtherComp :type "PrimitiveComponent Object Reference") (bSelfMoved :type Boolean) (HitLocation :type "Vector Structure") (HitNormal :type "Vector Structure") (NormalImpulse :type "Vector Structure") (Hit :type "HitResult Structure (by ref)"))
  ;[1 1 1] Apply damage on hit
  (if (`KismetSystemLibrary.DoesImplementInterface` Other "/Game/111Survival/BPI_Damageable.BPI_Damageable_C")
    (if (`self.ActorHasTag` Other "Friend")
      (`GameplayStatics.ApplyDamage` Other (`self.Damage`)))))

(event `self.FireExplosion.OnEndPlay`
  (params (Actor :type "Actor Object Reference") (EndPlayReason :type "EEndPlayReason Enum" :default "Destroyed"))
  (`self.K2_DestroyActor`))

(fn `UserConstructionScript`)