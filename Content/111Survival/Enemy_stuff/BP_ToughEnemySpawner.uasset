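; BP_ToughEnemySpawner periodically spawns big enemies while the game is Playing and spawning is enabled in the BP_StoreVars GameInstance.
; Tick drives a Delay that shrinks as round time runs out, using the shared spawn frequency limits scaled tenfold.
; After each delay it picks a random spawn-point class, finds that actor, spawns a random AI pawn at its transform and prints the result.
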(event `self.ReceiveTick`
  (params (DeltaSeconds :type "Float (single-precision)"))
  ;[1 1 1] Read GameState and act accordingly
  (bind _asbp_store_vars (cast `/Game/111Survival/BP_StoreVars` (`GameplayStatics.GetGameInstance`)))
  (switch `/Game/111Survival/EN_GameState` (`/Game/111Survival/BP_StoreVars.GameState` _asbp_store_vars)
    (:`NewEnumerator1`
      ;[1 1 1] Loop as long as Spawn New Enemies = true
      (if (`/Game/111Survival/BP_StoreVars.bSpawnNewEnemies` _asbp_store_vars)
        (bind _returnvalue (* (`/Game/111Survival/BP_StoreVars.EnemySpawnFreqSlowest` _asbp_store_vars) 10.0))
        (bind _returnvalue_2 (* (`/Game/111Survival/BP_StoreVars.EnemySpawnFreqFastest` _asbp_store_vars) 10.0))
        (`KismetSystemLibrary.Delay` (`KismetMathLibrary.FClamp` (+ (* (/ (- _returnvalue _returnvalue_2) 100.0) (* (/ (`/Game/111Survival/BP_StoreVars.RoundTimeLeft` _asbp_store_vars) (`/Game/111Survival/BP_StoreVars.WinTime` _asbp_store_vars)) 100.0)) _returnvalue_2) _returnvalue_2 _returnvalue))
        ;[1 1 1] Get random location for spawning
        (bind _returnvalue_3 (`GameplayStatics.GetActorOfClass` (`|GetArrayItem` (`self.EnemySpawnPoints`) (`KismetMathLibrary.RandomIntegerInRange` 0 (- (`KismetArrayLibrary.Array_Length` (`self.EnemySpawnPoints`)) 1)))))
        (bind _returnvalue_4 (`AIBlueprintHelperLibrary.SpawnAIFromClass` (`|GetArrayItem` (`self.EnemiesToSpawn`) (`KismetMathLibrary.RandomIntegerInRange` 0 (- (`KismetArrayLibrary.Array_Length` (`self.EnemiesToSpawn`)) 1))) null (`self.K2_GetActorLocation` _returnvalue_3) (`self.K2_GetActorRotation` _returnvalue_3) true null))
        (`/Engine/EditorBlueprintResources/StandardMacros.IsValid` _returnvalue_4
          (:`Is Valid`
            (`KismetSystemLibrary.PrintString` "Big enemy spawned"))
          (:`Is Not Valid`
            (`KismetSystemLibrary.PrintString` "Big enemy couldn't be spawned" true true (struct :`R` 1.0 :`G` 0.16251 :`B` 0.242219 :`A` 1.0) 3.0)))))))

(fn `UserConstructionScript`)