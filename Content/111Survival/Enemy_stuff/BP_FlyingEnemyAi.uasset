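; AI controller for a flying enemy that, every two seconds from BeginPlay, turns its pawn toward the stored door and moves to it.
; The door reference comes from the BP_StoreVars game instance.
; A FindTarget event traces toward the door and picks door, player or nearest wall from the hit.
; Nothing here calls FindTarget, and the ignore-list setup is disconnected.
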(event `FindTarget`
  ;[1 1 1] Find suitable target to run towards
  (bind _asbp_store_vars (cast `/Game/111Survival/BP_StoreVars` (`GameplayStatics.GetGameInstance`)))
  (bind _outhit (`KismetSystemLibrary.LineTraceSingle` (`self.K2_GetActorLocation` (`self.K2_GetPawn`)) (`self.K2_GetActorLocation` (`/Game/111Survival/BP_StoreVars.DoorInstance` _asbp_store_vars)) "TraceTypeQuery1" false (`self.IgnoredActors`) "None" true (struct :`R` 1.0 :`A` 1.0) (struct :`G` 1.0 :`A` 1.0) 1.0))
  (bind _returnvalue (`GameplayStatics.GetObjectClass` (`.HitActor` (`GameplayStatics.BreakHitResult` _outhit))))
  (if (`KismetMathLibrary.ClassIsChildOf` _returnvalue "/Game/111Survival/BP_Door.BP_Door_C")
    (`self.followDoor`)
    (elif (`KismetMathLibrary.ClassIsChildOf` _returnvalue "/Game/111Survival/BP_PlayerCharacter.BP_PlayerCharacter_C")
      (`self.followPlayer`)
      (else
        (`self.followWall`)))))

(event `followPlayer`
  (bind _returnvalue (`self.K2_GetPawn`))
  (bind (_returnvalue_roll _returnvalue_pitch _returnvalue_yaw) (`KismetMathLibrary.BreakRotator` (`KismetMathLibrary.FindLookAtRotation` (`self.K2_GetActorLocation` _returnvalue) (`self.K2_GetActorLocation` (`GameplayStatics.GetPlayerCharacter` 0)))))
  ;[1 1 1] Follow Player
  (`self.K2_SetActorRotation` _returnvalue (`KismetMathLibrary.MakeRotator` 0.0 0.0 _returnvalue_yaw) false)
  (`|AIMoveTo` (`self.K2_GetPawn`) (0.0 0.0 0.0) (`GameplayStatics.GetPlayerPawn` 0) (`self.AcceptanceRadius`)))

(event `self.ReceiveBeginPlay`
  (`KismetSystemLibrary.K2_SetTimer` null "followDoor" 2.0 true))

(event `followWall`
  (bind _returnvalue (`self.K2_GetPawn`))
  (bind _closestwall (`self.ClosestWall`))
  (bind _returnvalue_2 (`self.K2_GetActorLocation` _returnvalue))
  (bind (_returnvalue_roll _returnvalue_pitch _returnvalue_yaw) (`KismetMathLibrary.BreakRotator` (`KismetMathLibrary.FindLookAtRotation` _returnvalue_2 (`self.K2_GetActorLocation` _closestwall))))
  ;[1 1 1] Find closest wall, rotate to look at it, and move towards it. If there are no walls, follow door
  ;;[1 1 1] Find closest wall
  (bind _outactors (`GameplayStatics.GetAllActorsOfClass` "/Game/111Survival/BuildMode/Objects/BP_Wall.BP_Wall_C"))
  (for _array_element _outactors
    (bind _returnvalue_3 (`KismetMathLibrary.VSize` (- (`self.K2_GetActorLocation` _array_element) _returnvalue_2)))
    (if (< _returnvalue_3 (`self.ClosestDistance`))
      (set `self.ClosestDistance` _returnvalue_3)
      (set `self.ClosestWall` _array_element)))
  (`/Engine/EditorBlueprintResources/StandardMacros.IsValid` _closestwall
    (:`Is Valid`
      (`self.K2_SetActorRotation` _returnvalue (`KismetMathLibrary.MakeRotator` 0.0 0.0 _returnvalue_yaw) false)
      (`|AIMoveTo` (`self.K2_GetPawn`) (0.0 0.0 0.0) _closestwall (`self.AcceptanceRadius`)))
    (:`Is Not Valid`
      (`self.followDoor`))))

(event `followDoor`
  (bind _returnvalue (`self.K2_GetPawn`))
  ;[1 1 1] Follow Door
  (bind _asbp_store_vars (cast `/Game/111Survival/BP_StoreVars` (`GameplayStatics.GetGameInstance`)))
  (bind _doorinstance (`/Game/111Survival/BP_StoreVars.DoorInstance` _asbp_store_vars))
  (bind (_returnvalue_roll _returnvalue_pitch _returnvalue_yaw) (`KismetMathLibrary.BreakRotator` (`KismetMathLibrary.FindLookAtRotation` (`self.K2_GetActorLocation` _returnvalue) (`self.K2_GetActorLocation` _doorinstance))))
  (`self.K2_SetActorRotation` _returnvalue (`KismetMathLibrary.MakeRotator` 0.0 0.0 _returnvalue_yaw) false)
  (`|AIMoveTo` (`self.K2_GetPawn`) (0.0 0.0 0.0) _doorinstance (`self.AcceptanceRadius`)))

(fn `SetActorsToIgnore`
  ;[1 1 1] Set actors to ignore while finding target
  (bind _asbp_store_vars (cast `/Game/111Survival/BP_StoreVars` (`GameplayStatics.GetGameInstance`)))
  (set `self.IgnoredActors` (`/Game/111Survival/BP_StoreVars.IgnoredActors` _asbp_store_vars)))

(fn `UserConstructionScript`)