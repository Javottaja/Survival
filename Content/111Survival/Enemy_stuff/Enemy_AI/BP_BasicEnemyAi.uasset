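; AI controller for basic enemies in the survival game, choosing whether to chase the player, the door or a wall.
; A looping timer line-traces from the pawn toward the stored door to pick the target, but tough enemies always chase the player.
; When blocked by anything else, it moves to the closest wall, falling back to the door.
; A faster timer traces toward that wall and makes jumping enemies jump when close, then clears it.
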(event `FindTarget`
  (bind _returnvalue (`self.K2_GetPawn`))
  ;[1 1 1] Find suitable target to run towards
  (bind _asbp_store_vars (cast `/Game/111Survival/BP_StoreVars` (`GameplayStatics.GetGameInstance`)))
  (if (`KismetMathLibrary.ClassIsChildOf` (`GameplayStatics.GetObjectClass` _returnvalue) "/Game/111Survival/Enemy_stuff/Enemies/BP_ToughEnemy_Basic.BP_ToughEnemy_Basic_C")
    (`self.followPlayer` :!label _label)
    (else
      (bind _outhit (`KismetSystemLibrary.LineTraceSingle` (`self.K2_GetActorLocation` _returnvalue) (`self.K2_GetActorLocation` (`/Game/111Survival/BP_StoreVars.DoorInstance` _asbp_store_vars)) "TraceTypeQuery1" false (`self.IgnoredActors`) "None" true (struct :`R` 1.0 :`A` 1.0) (struct :`G` 1.0 :`A` 1.0) 0.1))
      (bind _returnvalue_2 (`GameplayStatics.GetObjectClass` (`.HitActor` (`GameplayStatics.BreakHitResult` _outhit))))
      (if (`KismetMathLibrary.ClassIsChildOf` _returnvalue_2 "/Game/111Survival/BP_Door.BP_Door_C")
        (`self.followDoor`)
        (elif (`KismetMathLibrary.ClassIsChildOf` _returnvalue_2 "/Game/111Survival/BP_PlayerCharacter.BP_PlayerCharacter_C")
          (goto _label)
          (else
            (`self.followWall`)))))))

(event `self.ReceiveBeginPlay`
  (`self.SetActorsToIgnore`)
  (`KismetSystemLibrary.K2_SetTimer` null "findTarget" 0.5 true)
  (`KismetSystemLibrary.K2_SetTimer` null "GetDistanceToClosestWall" 0.1 true))

(event `followPlayer`
  (bind _returnvalue (`self.K2_GetPawn`))
  (bind (_returnvalue_roll _returnvalue_pitch _returnvalue_yaw) (`KismetMathLibrary.BreakRotator` (`KismetMathLibrary.FindLookAtRotation` (`self.K2_GetActorLocation` _returnvalue) (`self.K2_GetActorLocation` (`GameplayStatics.GetPlayerCharacter` 0)))))
  ;[1 1 1] Follow Player
  (`self.K2_SetActorRotation` _returnvalue (`KismetMathLibrary.MakeRotator` 0.0 0.0 _returnvalue_yaw) false)
  (`|AIMoveTo` (`self.K2_GetPawn`) (0.0 0.0 0.0) (`GameplayStatics.GetPlayerPawn` 0) (`self.AcceptanceRadius`)))

(event `followDoor`
  (bind _returnvalue (`self.K2_GetPawn`))
  ;[1 1 1] Follow Door
  (bind _asbp_store_vars (cast `/Game/111Survival/BP_StoreVars` (`GameplayStatics.GetGameInstance`)))
  (bind _doorinstance (`/Game/111Survival/BP_StoreVars.DoorInstance` _asbp_store_vars))
  (bind (_returnvalue_roll _returnvalue_pitch _returnvalue_yaw) (`KismetMathLibrary.BreakRotator` (`KismetMathLibrary.FindLookAtRotation` (`self.K2_GetActorLocation` _returnvalue) (`self.K2_GetActorLocation` _doorinstance))))
  (`self.K2_SetActorRotation` _returnvalue (`KismetMathLibrary.MakeRotator` 0.0 0.0 _returnvalue_yaw) false)
  (`|AIMoveTo` (`self.K2_GetPawn`) (0.0 0.0 0.0) _doorinstance (`self.AcceptanceRadius`)))

(event `followWall`
  (bind _returnvalue (`self.K2_GetPawn`))
  (bind _closestwall (`self.ClosestWall`))
  (bind _returnvalue_2 (`self.K2_GetActorLocation` _returnvalue))
  (bind (_returnvalue_roll _returnvalue_pitch _returnvalue_yaw) (`KismetMathLibrary.BreakRotator` (`KismetMathLibrary.FindLookAtRotation` _returnvalue_2 (`self.K2_GetActorLocation` _closestwall))))
  ;[1 1 1] Find closest wall, rotate to look at it, and move towards it. If there are no walls, follow door
  ;;[1 1 1] Find closest wall
  (bind _outactors (`GameplayStatics.GetAllActorsOfClass` "/Game/111Survival/BuildMode/Objects/BP_Wall.BP_Wall_C"))
  (for _array_element _outactors
    (bind _returnvalue_3 (`KismetMathLibrary.VSize` (- (`self.K2_GetActorLocation` _array_element) _returnvalue_2)))
    (if (< _returnvalue_3 (`self.ClosestDistance`))
      (set `self.ClosestDistance` _returnvalue_3)
      (set `self.ClosestWall` _array_element)))
  (`/Engine/EditorBlueprintResources/StandardMacros.IsValid` _closestwall
    (:`Is Valid`
      (`self.K2_SetActorRotation` _returnvalue (`KismetMathLibrary.MakeRotator` 0.0 0.0 _returnvalue_yaw) false)
      (`|AIMoveTo` (`self.K2_GetPawn`) (0.0 0.0 0.0) _closestwall (`self.AcceptanceRadius`)))
    (:`Is Not Valid`
      (`self.followDoor`))))

(event `GetDistanceToClosestWall`
  (bind _returnvalue (`self.K2_GetPawn`))
  (bind _closestwall (`self.ClosestWall`))
  ;[1 1 1] Get distance to closest wall. When under JumpTriggerTreshold, jump and clear ClosestWall variable
  (`/Engine/EditorBlueprintResources/StandardMacros.IsValid` _closestwall
    (:`Is Valid`
      (bind _outhit (`KismetSystemLibrary.LineTraceSingle` :`Start` (`self.K2_GetActorLocation` _returnvalue) :`End` (`KismetMathLibrary.MakeVector` (.x (`self.K2_GetActorLocation` _closestwall)) (.y (`self.K2_GetActorLocation` _closestwall)) (+ (.z (`self.K2_GetActorLocation` _closestwall)) 100.0)) :`TraceChannel` "TraceTypeQuery1" :`DrawDebugType` "ForDuration" :`DrawTime` 0.05))
      (`/Engine/EditorBlueprintResources/StandardMacros.IsValid` (`.HitActor` (`GameplayStatics.BreakHitResult` _outhit))
        (:`Is Valid`
          (if (`KismetMathLibrary.ClassIsChildOf` (`GameplayStatics.GetObjectClass` (`.HitActor` (`GameplayStatics.BreakHitResult` _outhit))) "/Game/111Survival/BuildMode/Objects/BP_Wall.BP_Wall_C")
            (if (<= (`.Distance` (`GameplayStatics.BreakHitResult` _outhit)) (`self.JumpTriggerTreshold`))
              (bind _asbp_basic_enemy_jumping (cast `/Game/111Survival/Enemy_stuff/Enemies/BP_BasicEnemy_Jumping` _returnvalue))
              (if (`Character.CanJump` _asbp_basic_enemy_jumping)
                (`Character.Jump` _asbp_basic_enemy_jumping)
                (set `self.ClosestWall` null)))))))))

(fn `SetActorsToIgnore`
  ;[1 1 1] Set actors to ignore while finding target
  (bind _asbp_store_vars (cast `/Game/111Survival/BP_StoreVars` (`GameplayStatics.GetGameInstance`)))
  (set `self.IgnoredActors` (`/Game/111Survival/BP_StoreVars.IgnoredActors` _asbp_store_vars)))

(fn `UserConstructionScript`)