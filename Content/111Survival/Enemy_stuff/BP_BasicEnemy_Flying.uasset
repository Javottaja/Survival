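; BP_BasicEnemy_Flying is a flying enemy that shoots at the door when within range.
; A looping one-second timer line-traces from the enemy to the DoorInstance stored in the BP_StoreVars game instance.
; If the trace hits a BP_Door within the firing distance, it calls FireShot with the direction toward that actor.
; The firing distance is meant to sit inside the FlyingEnemyAi acceptance radius.
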(event `self.ReceiveBeginPlay`
  (`KismetSystemLibrary.K2_SetTimer` null "GetDistanceToDoor" 1.0 true))

(event `GetDistanceToDoor`
  ;[1 1 1] When FlyingEnemyAi AcceptanceRadius = 900, we want OutHitDistance to be less than 800
  (bind _asbp_store_vars (cast `/Game/111Survival/BP_StoreVars` (`GameplayStatics.GetGameInstance`)))
  (bind _outhit (`KismetSystemLibrary.LineTraceSingle` :`Start` (`self.K2_GetActorLocation`) :`End` (`self.K2_GetActorLocation` (`/Game/111Survival/BP_StoreVars.DoorInstance` _asbp_store_vars)) :`TraceChannel` "TraceTypeQuery1" :`DrawTime` 1.0))
  (`/Engine/EditorBlueprintResources/StandardMacros.IsValid` (`.HitActor` (`GameplayStatics.BreakHitResult` _outhit))
    (:`Is Valid`
      (if (and (<= (`.Distance` (`GameplayStatics.BreakHitResult` _outhit)) 800.0) (`KismetMathLibrary.ClassIsChildOf` (`GameplayStatics.GetObjectClass` (`.HitActor` (`GameplayStatics.BreakHitResult` _outhit))) "/Game/111Survival/BP_Door.BP_Door_C"))
        ;[1 1 1] Rotate and shoot
        (`self.FireShot` (`KismetMathLibrary.Conv_RotatorToVector` (`KismetMathLibrary.FindLookAtRotation` (`self.K2_GetActorLocation`) (`self.K2_GetActorLocation` (`.HitActor` (`GameplayStatics.BreakHitResult` _outhit))))))))))

(fn `UserConstructionScript`
  (`parent.UserConstructionScript`))