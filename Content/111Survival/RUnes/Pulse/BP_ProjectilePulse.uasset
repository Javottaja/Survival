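; Pulse rune projectile: a blast whose collision sphere grows every frame over its lifespan.
; On BeginPlay it derives a per-frame increment from lifespan, the game instance's FPS (capped) and a growth multiplier.
; The multiplier is fixed for owned (turret-spawned) pulses or one firing mode, otherwise scaled by weapon charge time.
; Tick enlarges the sphere, then sizes a box from its bounds to scale the flat cylinder visual.
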(event `self.ReceiveBeginPlay`
  (`self.GetCurrentFPS`)
  (`self.Initialize`))

(event `self.ReceiveTick`
  (params (DeltaSeconds :type "Float (single-precision)"))
  (`self.GrowProjectileSize`))

(fn `GetCurrentFPS`
  (bind _asbp_store_vars (cast `/Game/111Survival/BP_StoreVars` (`GameplayStatics.GetGameInstance`)))
  (set `self.CurrentFPS` (`/Game/111Survival/BP_StoreVars.CurrentFPS` _asbp_store_vars)))

(fn `GrowProjectileSize`
  (bind _initialsize (`self.InitialSize`))
  (bind _projectilecollision (`self.ProjectileCollision`))
  (bind (_returnvalue_x _returnvalue_y _returnvalue_z) (`KismetMathLibrary.BreakVector` (`BoxComponent.GetScaledBoxExtent` (`self.Box`))))
  (bind (_origin _boxextent _sphereradius) (`KismetSystemLibrary.GetComponentBounds` (`self.ProjectileCollision`)))
  ;[1 1 1] Set radius of the actual collision
  (`SphereComponent.SetSphereRadius` _projectilecollision (+ (`SphereComponent.SphereRadius` _projectilecollision) (`self.SizeIncrementPerFrame`)) true)
  ;[1 1 1] Calculate bounds for visuals of the projectile
  (`BoxComponent.SetBoxExtent` (`self.Box`) (`KismetMathLibrary.MakeVector` _sphereradius _sphereradius 0.05) false)
  ;[1 1 1] Set size of the visuals, based on calculated bounds
  (`SceneComponent.SetWorldScale3D` (`self.Cylinder`) (`KismetMathLibrary.MakeVector` (/ _returnvalue_x _initialsize) (/ _returnvalue_y _initialsize) _returnvalue_z)))

(fn `Initialize`
  ;[1 1 1] Set growth multiplier, so we can calculate target size
  ; (this actor has an owner if a Turret spawned it)
  (`/Engine/EditorBlueprintResources/StandardMacros.IsValid` (`self.GetOwner`)
    (:`Is Valid`
      (set `self.GrowthMultiplier` 2.0 :!label _label))
    (:`Is Not Valid`
      (if (`|EnumEquality` (`self.FiringMode`) "NewEnumerator0")
        (goto _label)
        (else
          (bind _asbp_store_vars (cast `/Game/111Survival/BP_StoreVars` (`GameplayStatics.GetGameInstance`)))
          (set `self.GrowthMultiplier` (* (`/Game/111Survival/BP_StoreVars.WeaponChargeTime` _asbp_store_vars) 2.0))))))
  ;[1 1 1] Target size of pulse blast
  (set `self.TargetSize` (* (`SphereComponent.SphereRadius` (`self.ProjectileCollision`)) (`self.GrowthMultiplier`)))
  ;[1 1 1] How many frames we have to grow the pulse blast
  (set `self.FrameCount` (* (`KismetMathLibrary.FClamp` (`self.CurrentFPS`) 0.0 60.0) (`self.InitialLifeSpan`)))
  ;[1 1 1] Calculate size increment per frame
  (set `self.SizeIncrementPerFrame` (/ (`self.TargetSize`) (`self.FrameCount`)))
  ;[1 1 1] Set initial radius
  (`SphereComponent.SetSphereRadius` (`self.ProjectileCollision`) (`self.InitialSize`) true))

(fn `UserConstructionScript`
  (`parent.UserConstructionScript`))