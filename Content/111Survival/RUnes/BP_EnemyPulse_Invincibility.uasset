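; BP_EnemyPulse_Invincibility is an enemy pulse variant, filed under Runes, that grants invincibility to regular enemies.
; Its DoDamage function deals no damage itself: it filters the passed actor for the Enemy tag, excludes Boss, casts to BP_BasicEnemy and calls TriggerInvincibility.
; The event graph holds only disabled stub events, so nothing in this Blueprint calls DoDamage.
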(fn `DoDamage`
  (params (OtherActor :type "Actor Object Reference"))
  ;[1 1 1] IS enemy and IS NOT boss
  (if (`self.ActorHasTag` OtherActor "Enemy")
    (if (not (`self.ActorHasTag` OtherActor "Boss"))
      ;[1 1 1] Do the thing
      (bind _asbp_basic_enemy (cast `/Game/111Survival/Enemy_stuff/Enemies/BP_BasicEnemy` OtherActor))
      (`/Game/111Survival/Enemy_stuff/Enemies/BP_BasicEnemy.TriggerInvincibility` _asbp_basic_enemy))))

(fn `UserConstructionScript`
  (`parent.UserConstructionScript`))