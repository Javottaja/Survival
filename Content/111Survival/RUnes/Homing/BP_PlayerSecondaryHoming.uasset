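; Player secondary homing projectile that bounces between the player and tagged BP_BasicEnemy actors.
; On movement activation it homes on the nearest enemy, dropping the last target's stored index from each search list.
; Overlapping an enemy redirects homing to the player, and overlapping the player triggers a new lock-on.
; A looping timer re-locks when the target is no longer valid, despite the inverted name of CheckIfTargetIsInvalidated.
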(event `self.ReceiveBeginPlay`
  (`ActorComponent.Activate` (`self.ProjectileMovement`) false)
  (`KismetSystemLibrary.K2_SetTimerDelegate` (delegate `RevalidateTarget`) 1.0 true))

(event `Lock On`
  (bind _homingtarget (`self.FindHomingTarget`))
  (set `ProjectileMovementComponent.HomingTargetComponent` _homingtarget (`self.ProjectileMovement`)))

(event `RevalidateTarget`
  (bind _hasvalidtarget (`self.CheckIfTargetIsInvalidated`))
  (if (not _hasvalidtarget)
    (`self.Lock On` :!label _label)))

(event `self.ProjectileMovement.OnComponentActivated`
  (params (Component :type "ActorComponent Object Reference") (bReset :type Boolean))
  (goto _label))

(event `self.ProjectileCollision.OnComponentBeginOverlap`
  (params (OverlappedComponent :type "PrimitiveComponent Object Reference") (OtherActor :type "Actor Object Reference") (OtherComp :type "PrimitiveComponent Object Reference") (OtherBodyIndex :type Integer) (bFromSweep :type Boolean) (SweepResult :type "HitResult Structure (by ref)"))
  (if (`self.ActorHasTag` OtherActor "Player")
    (`KismetSystemLibrary.PrintString` "Hit Player")
    (goto _label)
    (elif (`self.ActorHasTag` OtherActor "Enemy")
      (`KismetSystemLibrary.PrintString` "Hit enemy")
      (`self.ReturnToPlayer`))))

(fn `CheckIfTargetIsInvalidated`
  (returns (HasValidTarget :type Boolean))
  (return (`KismetSystemLibrary.IsValid` (`self.HomingTarget`))))

(fn `FindHomingTarget`
  (returns (HomingTarget :type "SceneComponent Object Reference"))
  (bind _homingtarget (`self.HomingTarget`))
  (set `self.ClosestDistance` 1000000000.0)
  (bind _outactors (`GameplayStatics.GetAllActorsOfClassWithTag` "/Game/111Survival/Enemy_stuff/Enemies/BP_BasicEnemy.BP_BasicEnemy_C" "Enemy"))
  (bind _output_get (set `self.EnemyList` _outactors))
  (`KismetArrayLibrary.Array_Remove` _output_get (`self.HomingTargetIndex`))
  (for (_array_element _array_index) (`self.EnemyList`)
    (bind _returnvalue (`KismetMathLibrary.VSize` (- (`self.K2_GetActorLocation` _array_element) (`self.K2_GetActorLocation`))))
    (if (< _returnvalue (`self.ClosestDistance`))
      (set `self.ClosestDistance` _returnvalue)
      (set `self.HomingTarget` _array_element)
      (set `self.HomingTargetIndex` _array_index)))
  (`/Engine/EditorBlueprintResources/StandardMacros.IsValid` _homingtarget
    (:`Is Valid`
      (return (`self.GetComponentByClass` _homingtarget "/Script/Engine.SceneComponent")))))

(fn `ReturnToPlayer`
  (set `ProjectileMovementComponent.HomingTargetComponent` (`self.GetComponentByClass` (`GameplayStatics.GetPlayerCharacter` 0) "/Script/Engine.SceneComponent") (`self.ProjectileMovement`)))

(fn `UserConstructionScript`
  (`parent.UserConstructionScript`))