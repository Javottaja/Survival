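; Homing projectile variant for the rune system that steers toward nearby enemies.
; While its movement component is active, it re-runs LockOn every half second to set the homing target component.
; Target search scans BP_BasicEnemy actors tagged Enemy for the one nearest the projectile.
; ClosestDistance is not reset between searches, so the target changes only when an enemy beats the stored distance.
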(event `Lock On`
  (bind _homingtarget (`self.FindHomingTarget`))
  (set `ProjectileMovementComponent.HomingTargetComponent` _homingtarget (`self.ProjectileMovement`)))

(event `self.ProjectileMovement.OnComponentActivated`
  (params (Component :type "ActorComponent Object Reference") (bReset :type Boolean))
  (`self.Lock On` :!label _label)
  (`KismetSystemLibrary.Delay` 0.5)
  (goto _label))

(fn `FindHomingTarget`
  (returns (HomingTarget :type "SceneComponent Object Reference"))
  (bind _homingtarget (`self.HomingTarget`))
  (bind _outactors (`GameplayStatics.GetAllActorsOfClassWithTag` "/Game/111Survival/Enemy_stuff/Enemies/BP_BasicEnemy.BP_BasicEnemy_C" "Enemy"))
  (for _array_element _outactors
    (bind _returnvalue (`KismetMathLibrary.VSize` (- (`self.K2_GetActorLocation` _array_element) (`self.K2_GetActorLocation`))))
    (if (< _returnvalue (`self.ClosestDistance`))
      (set `self.ClosestDistance` _returnvalue)
      (set `self.HomingTarget` _array_element)))
  (`/Engine/EditorBlueprintResources/StandardMacros.IsValid` _homingtarget
    (:`Is Valid`
      (return (`self.GetComponentByClass` _homingtarget "/Script/Engine.SceneComponent")))))

(fn `UserConstructionScript`
  (`parent.UserConstructionScript`))