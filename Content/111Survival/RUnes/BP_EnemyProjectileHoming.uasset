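; Enemy homing projectile that steers toward the BP_Door actor and damages what it overlaps.
; When ProjectileMovement activates, a repeating half-second loop finds the door and sets one of its scene components as the homing target.
; On overlap it passes the other actor to DoDamageAndDestroyProjectile to apply damage and remove itself.
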(event `self.ReceiveActorBeginOverlap`
  (params (OtherActor :type "Actor Object Reference"))
  (`self.DoDamageAndDestroyProjectile` OtherActor))

(event `Lock On`
  (bind _homingtarget (`self.FindHomingTarget`))
  (set `ProjectileMovementComponent.HomingTargetComponent` _homingtarget (`self.ProjectileMovement`)))

(event `self.ProjectileMovement.OnComponentActivated`
  (params (Component :type "ActorComponent Object Reference") (bReset :type Boolean))
  (`self.Lock On` :!label _label)
  (`KismetSystemLibrary.Delay` 0.5)
  (goto _label))

(fn `FindHomingTarget`
  (returns (HomingTarget :type "SceneComponent Object Reference"))
  (bind _returnvalue (`GameplayStatics.GetActorOfClass` "/Game/111Survival/BP_Door.BP_Door_C"))
  (`/Engine/EditorBlueprintResources/StandardMacros.IsValid` _returnvalue
    (:`Is Valid`
      (set `self.HomingTarget` _returnvalue)
      (return (`self.GetComponentByClass` (`self.HomingTarget`) "/Script/Engine.SceneComponent")))))

(fn `UserConstructionScript`
  (`parent.UserConstructionScript`))