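; Base projectile for shots fired by the player or by defenses such as turrets, with a homing child.
; Construction scales damage and other stats from its owner: turret secondary rune and damage penalty, or player passive bonus and active powerup.
; On overlap it damages BPI_Damageable enemies, optionally tagged friendlies, and destroys itself unless piercing; defenses can block it.
; Damage-over-time shots repeat damage through a Delay loop without rechecking overlap.
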(event `self.ProjectileCollision.OnComponentBeginOverlap`
  (params (OverlappedComponent :type "PrimitiveComponent Object Reference") (OtherActor :type "Actor Object Reference") (OtherComp :type "PrimitiveComponent Object Reference") (OtherBodyIndex :type Integer) (bFromSweep :type Boolean) (SweepResult :type "HitResult Structure (by ref)"))
  (`self.CheckIfOverlappedDefense` OtherActor)
  (`/Engine/EditorBlueprintResources/StandardMacros.IsValid` OtherActor
    (:`Is Valid`
      (`self.DoDamage` OtherActor :!label _label)
      ;[1 1 1] If projectile deals damage over time, keep doing damage
      (`/Engine/EditorBlueprintResources/StandardMacros.IsValid` self
        (:`Is Valid`
          (if (`self.DealsDOT`)
            (`KismetSystemLibrary.Delay` 0.2)
            (goto _label)))))))

(fn `CalculatePowerupMultipliers`
  (params (Modifiers :type "/Game/111Survival/Powerups/S_PowerupMultipliers Structure"))
  (set `self.Damage` (* (`self.Damage`) Modifiers_DamageMultiplier_2_5E6529D24EAB318BCBF529B5F12CE6B9))
  (set `self.FireRate` (* (`self.FireRate`) Modifiers_FireRateMultiplier_5_5DC216084D1FBB273F947A837612169A))
  (set `self.ProjectileTargetSize` (* (`self.ProjectileTargetSize`) Modifiers_ProjectileSizeMultiplier_10_D7BEE67D498A1FF8A3B4F0BFFE791312)))

(fn `CheckIfOverlappedDefense`
  (params (OtherActor :type "Actor Object Reference"))
  (`/Engine/EditorBlueprintResources/StandardMacros.IsValid` OtherActor
    (:`Is Valid`
      (if (`self.IsStoppedByDefenses`)
        (if (`KismetMathLibrary.ClassIsChildOf` (`GameplayStatics.GetObjectClass` OtherActor) "/Game/111Survival/BuildMode/Objects/BP_DefenseBase.BP_DefenseBase_C")
          (`self.K2_DestroyActor`))))))

(fn `CheckSecondaryRune`
  (bind _returnvalue (`self.GetOwner`))
  (`/Engine/EditorBlueprintResources/StandardMacros.IsValid` _returnvalue
    (:`Is Valid`
      (if (`KismetMathLibrary.ClassIsChildOf` (`GameplayStatics.GetObjectClass` _returnvalue) "/Game/111Survival/BuildMode/Objects/BP_Turret.BP_Turret_C")
        (bind _asbp_turret (cast `/Game/111Survival/BuildMode/Objects/BP_Turret` _returnvalue))
        (bind _secondaryrune (`/Game/111Survival/BuildMode/Objects/BP_Turret.SecondaryRune` _asbp_turret))
        (if (`KismetSystemLibrary.IsValidClass` _secondaryrune)
          (bind (_damagefactor _fireratefactor) (defaults `Object` (`.TurretSecondary_7_0C28B3164FA72F9AA87B4E92AB1D5C11` (break `/Game/111Survival/RUnes/S_RuneContent` (`.RuneContents` (defaults `Object` _secondaryrune))))))
          (set `self.Damage` (* (`self.Damage`) _damagefactor))
          (set `self.FireRateFromTurret` (* (`self.FireRateFromTurret`) _fireratefactor)))))))

(fn `CheckWhoFiredMe`
  ;[1 1 1] Turret fired this projectile
  (if (`KismetMathLibrary.ClassIsChildOf` (`GameplayStatics.GetObjectClass` (`self.GetOwner`)) "/Game/111Survival/BuildMode/Objects/BP_DefenseBase.BP_DefenseBase_C")
    ;[1 1 1] Turrets deal less damage
    (set `self.Damage` (* (`self.Damage`) 0.25))
    ;[1 1 1] If this is a homing projectile fired by turret, it isn't stopped by defenses
    (if (`KismetMathLibrary.ClassIsChildOf` (`GameplayStatics.GetObjectClass` self) "/Game/111Survival/RUnes/Homing/BP_ProjectileHoming.BP_ProjectileHoming_C")
      (set `self.IsStoppedByDefenses` false))
    (else
      ;[1 1 1] Modify damage based on passive bonus
      (bind _asbp_player_character (cast `/Game/111Survival/BP_PlayerCharacter` (`self.GetOwner`)))
      (set `self.Damage` (* (`self.Damage`) (`.BaseDamageModifier_28_66C2B306444EBE97445EA49AF9239912` (break `/Game/111Survival/S_PassiveBonusLevels` (`/Game/111Survival/BP_PlayerCharacter.PassiveBonuses` _asbp_player_character))))))))

(fn `DoDamage`
  (params (OtherActor :type "Actor Object Reference"))
  (bind _damage (`self.Damage`))
  (if (`self.DamagesEverything`)
    (`/Engine/EditorBlueprintResources/StandardMacros.IsValid` OtherActor
      (:`Is Valid`
        ;[1 1 1] Check if target is valid
        (if (`KismetSystemLibrary.DoesImplementInterface` OtherActor "/Game/111Survival/BPI_Damageable.BPI_Damageable_C")
          ;[1 1 1] Damage everything. 10 dmg to friendlies, real damage to enemies
          (if (`self.ActorHasTag` OtherActor "Enemy")
            (`GameplayStatics.ApplyDamage` OtherActor _damage)
            ;[1 1 1] Destroy projectile if it doesn't go through enemies
            (if (not (`self.GoesThroughEnemies`)) :!label _label
              (`self.K2_DestroyActor`))
            (elif (and (`self.ActorHasTag` OtherActor "Friend") (`self.ActorHasTag` OtherActor "CanTakeFriendlyDamage"))
              (`GameplayStatics.ApplyDamage` OtherActor 10.0)
              (goto _label))))))
    (else
      (`/Engine/EditorBlueprintResources/StandardMacros.IsValid` OtherActor
        (:`Is Valid`
          ;[1 1 1] Check if target is valid
          (if (and (`KismetSystemLibrary.DoesImplementInterface` OtherActor "/Game/111Survival/BPI_Damageable.BPI_Damageable_C") (`self.ActorHasTag` OtherActor "Enemy"))
            (`GameplayStatics.ApplyDamage` OtherActor _damage)
            (goto _label)))))))

(fn `DoDamageAndDestroyProjectile`
  (params (OtherActor :type "Actor Object Reference"))
  (`/Engine/EditorBlueprintResources/StandardMacros.IsValid` OtherActor
    (:`Is Valid`
      ;[1 1 1] Apply damage on hit
      (if (and (`KismetSystemLibrary.DoesImplementInterface` OtherActor "/Game/111Survival/BPI_Damageable.BPI_Damageable_C") (`self.ActorHasTag` OtherActor "Enemy"))
        (`GameplayStatics.ApplyDamage` OtherActor (`self.Damage`))
        (`self.K2_DestroyActor`)))))

(fn `UserConstructionScript`
  (`|ExecutionSequence`
    (:`then_0`
      (`self.CheckSecondaryRune`))
    (:`then_1`
      (`self.CheckWhoFiredMe`))
    (:`then_2`
      ;[1 1 1] If powerup is active
      (bind _asbp_player_character (cast `/Game/111Survival/BP_PlayerCharacter` (`self.GetOwner`)))
      (if (`/Game/111Survival/BP_PlayerCharacter.IsPowerupActive` _asbp_player_character)
        (`self.CalculatePowerupMultipliers` (`/Game/111Survival/BP_PlayerCharacter.PowerUpModifiers` _asbp_player_character))))))