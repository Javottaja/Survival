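; Enemy projectile that acts as a pulse blast, expanding its collision sphere from an initial radius to a target size.
; On BeginPlay it reads the FPS from BP_StoreVars on the game instance, clamps it and multiplies by lifespan to derive a fixed per-frame increment.
; Each Tick grows the sphere until it reaches the target, then sizes a Box from its bounds to scale the flat Cylinder visual, a workaround marked PURKKA.
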(event `self.ReceiveBeginPlay`
  (`self.GetCurrentFPS`)
  (`self.Initialize`))

(event `self.ReceiveTick`
  (params (DeltaSeconds :type "Float (single-precision)"))
  (`self.GrowPulseSize`))

(fn `GetCurrentFPS`
  (bind _asbp_store_vars (cast `/Game/111Survival/BP_StoreVars` (`GameplayStatics.GetGameInstance`)))
  (set `self.CurrentFPS` (`/Game/111Survival/BP_StoreVars.CurrentFPS` _asbp_store_vars)))

(fn `GrowPulseSize`
  (bind _pulseinitialsize (`self.PulseInitialSize`))
  (bind _projectilecollision (`self.ProjectileCollision`))
  (bind (_returnvalue_x _returnvalue_y _returnvalue_z) (`KismetMathLibrary.BreakVector` (`BoxComponent.GetScaledBoxExtent` (`self.Box`))))
  (bind _sphereradius (`SphereComponent.SphereRadius` _projectilecollision))
  (bind _returnvalue (* (`.SphereRadius` (`KismetSystemLibrary.GetComponentBounds` (`self.ProjectileCollision`))) 1.25))
  (if (< _sphereradius (`self.PulseTargetSize`))
    ;[1 1 1] Set radius of the actual collision
    (`SphereComponent.SetSphereRadius` _projectilecollision (+ _sphereradius (`self.SizeIncrementPerFrame`)) true)
    ;[1 1 1] Calculate bounds for visuals of the projectile
    (`BoxComponent.SetBoxExtent` (`self.Box`) (`KismetMathLibrary.MakeVector` _returnvalue _returnvalue 0.05) false)
    ;[1 1 1] Set size of the visuals, based on calculated bounds
    (`SceneComponent.SetWorldScale3D` (`self.Cylinder`) (`KismetMathLibrary.MakeVector` (/ _returnvalue_x _pulseinitialsize) (/ _returnvalue_y _pulseinitialsize) _returnvalue_z))))

(fn `Initialize`
  ;[1 1 1] How many frames we have to grow the pulse blast
  (set `self.FrameCount` (* (`KismetMathLibrary.FClamp` (`self.CurrentFPS`) 0.0 60.0) (`self.InitialLifeSpan`)))
  ;[1 1 1] Calculate size increment per frame
  (set `self.SizeIncrementPerFrame` (/ (`self.PulseTargetSize`) (`self.FrameCount`)))
  ;[1 1 1] Initial radius
  (`SphereComponent.SetSphereRadius` (`self.ProjectileCollision`) (`self.PulseInitialSize`) true))

(fn `UserConstructionScript`
  (`parent.UserConstructionScript`))