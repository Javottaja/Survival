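; BP_ProjectilePulse is a pulse projectile whose cylinder grows while it is alive and damages actors it overlaps.
; On BeginPlay it sets its lifespan from the projectile override stored in the BP_StoreVars game instance.
; Each Tick multiplies the cylinder's world scale by ProjectileSizeIncrement, so growth compounds and depends on frame rate.
; Cylinder overlaps pass the other actor straight to DoDamage, with no filtering in this graph.
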(event `self.ReceiveBeginPlay`
  (bind _asbp_store_vars (cast `/Game/111Survival/BP_StoreVars` (`GameplayStatics.GetGameInstance`)))
  (`self.SetLifeSpan` (`/Game/111Survival/BP_StoreVars.ProjectileLifeSpanOverride` _asbp_store_vars)))

(event `self.ReceiveTick`
  (params (DeltaSeconds :type "Float (single-precision)"))
  (`SceneComponent.SetWorldScale3D` (`self.Cylinder`) (* (`SceneComponent.K2_GetComponentScale` (`self.Cylinder`)) (`self.ProjectileSizeIncrement`))))

(event `self.Cylinder.OnComponentBeginOverlap`
  (params (OverlappedComponent :type "PrimitiveComponent Object Reference") (OtherActor :type "Actor Object Reference") (OtherComp :type "PrimitiveComponent Object Reference") (OtherBodyIndex :type Integer) (bFromSweep :type Boolean) (SweepResult :type "HitResult Structure (by ref)"))
  (`self.DoDamage` OtherActor))

(fn `UserConstructionScript`
  (`parent.UserConstructionScript`))