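; Base enemy projectile that damages damageable actors it overlaps, hitting both friends and other enemies.
; A collision overlap calls DoDamage, which filters targets by BPI_Damageable and actor tag, applying base damage to "Friend" actors and a tenfold amount to "Enemy" actors.
; The projectile destroys itself after a hit unless GoesThroughEnemies is set.
; A separate DoDamageAndDestroyProjectile function, not called here, damages only friends and always destroys the projectile.
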(event `self.ProjectileCollision.OnComponentBeginOverlap`
  (params (OverlappedComponent :type "PrimitiveComponent Object Reference") (OtherActor :type "Actor Object Reference") (OtherComp :type "PrimitiveComponent Object Reference") (OtherBodyIndex :type Integer) (bFromSweep :type Boolean) (SweepResult :type "HitResult Structure (by ref)"))
  (`/Engine/EditorBlueprintResources/StandardMacros.IsValid` OtherActor
    (:`Is Valid`
      (`self.DoDamage` OtherActor))))

(fn `DoDamage`
  (params (OtherActor :type "Actor Object Reference"))
  (bind _returnvalue (`KismetSystemLibrary.DoesImplementInterface` OtherActor "/Game/111Survival/BPI_Damageable.BPI_Damageable_C"))
  (bind _damage (`self.Damage`))
  (`|ExecutionSequence`
    (:`then_0`
      ;[1 1 1] Apply damage on hit
      (if (and (`self.ActorHasTag` OtherActor "Friend") _returnvalue)
        (`GameplayStatics.ApplyDamage` OtherActor _damage)
        ;[1 1 1] Destroy projectile if it doesn't go through enemies
        (if (not (`self.GoesThroughEnemies`)) :!label _label
          (`self.K2_DestroyActor`))))
    (:`then_1`
      (if (and _returnvalue (`self.ActorHasTag` OtherActor "Enemy"))
        (`GameplayStatics.ApplyDamage` OtherActor (* _damage 10.0))
        (goto _label)))))

(fn `DoDamageAndDestroyProjectile`
  (params (OtherActor :type "Actor Object Reference"))
  (`/Engine/EditorBlueprintResources/StandardMacros.IsValid` OtherActor
    (:`Is Valid`
      ;[1 1 1] Apply damage on hit
      (if (and (`KismetSystemLibrary.DoesImplementInterface` OtherActor "/Game/111Survival/BPI_Damageable.BPI_Damageable_C") (`self.ActorHasTag` OtherActor "Friend"))
        (`GameplayStatics.ApplyDamage` OtherActor (`self.Damage`))
        (`self.K2_DestroyActor`)))))

(fn `UserConstructionScript`)