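; BP_Wall is a destructible, upgradable wall for build mode that updates a floating health bar when damaged and destroys itself at zero health.
; On BeginPlay it writes its level to the nearest WallGridManager cell and the game-instance database, then plays a spawn animation on that level's mesh.
; Upgrading, gated by game state, focuses the camera and opens UI_LevelUp.
; DisableWall applies pulse material and removes nav blocking; EnableWall has the grid manager rebuild it.
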(event `self.ReceiveAnyDamage`
  (params (Damage :type "Float (single-precision)") (DamageType :type "DamageType Object Reference") (InstigatedBy :type "Controller Object Reference") (DamageCauser :type "Actor Object Reference"))
  ;[1 1 1] Take damage. If Health drops to 0, lose the game
  (bind _output_get (set `self.HealthCurrent` (`KismetMathLibrary.FClamp` (- (`self.HealthCurrent`) Damage) 0.0 (`self.HealthMax`))))
  (bind _asui_floating_health_bar (cast `/Game/111Survival/UI/UI_FloatingHealthBar` (`WidgetComponent.GetUserWidgetObject` (`self.WallHealth`))))
  (set `/Game/111Survival/UI/UI_FloatingHealthBar.HealthCurrent` _output_get _asui_floating_health_bar)
  (`/Game/111Survival/UI/UI_FloatingHealthBar.UpdateHealth` _asui_floating_health_bar)
  (if (<= _output_get 0.0)
    (`self.K2_DestroyActor`)))

(event `self.ReceiveBeginPlay`
  (bind _walllevel (`self.WallLevel`))
  (`|ExecutionSequence`
    (:`then_0`
      ;[1 1 1] Set health parameters for BuildingHealth widget
      (bind _asui_floating_health_bar (cast `/Game/111Survival/UI/UI_FloatingHealthBar` (`WidgetComponent.GetUserWidgetObject` (`self.WallHealth`))))
      (set `/Game/111Survival/UI/UI_FloatingHealthBar.HealthMax` (`self.HealthMax`) _asui_floating_health_bar)
      (set `/Game/111Survival/UI/UI_FloatingHealthBar.HealthCurrent` (`self.HealthCurrent`) _asui_floating_health_bar))
    (:`then_1`
      ;[1 1 1] Set the level of the wall into local and persistent database
      (bind _returnvalue (`GameplayStatics.GetActorOfClass` "/Game/111Survival/BuildMode/Grid/WallGridManager.WallGridManager_C"))
      (bind _outputvector (`/Game/111Survival/BuildMode/Grid/WallGridManager.GetClosestGridCell` _returnvalue (`SceneComponent.K2_GetComponentLocation` (`self.OriginPoint`))))
      (setmembers `/Game/111Survival/BuildMode/Grid/S_WallGridContentData` :`StructRef` (`/Game/111Survival/BuildMode/Grid/WallGridCell.GridCellContentData` _outputvector) :`WallLevel` _walllevel)
      (bind _asbp_store_vars (cast `/Game/111Survival/BP_StoreVars` (`GameplayStatics.GetGameInstance`)))
      (setmembers `/Game/111Survival/BuildMode/Grid/S_WallGridContentData` :`StructRef` (`|GetArrayItem` (`/Game/111Survival/BP_StoreVars.WallGridContentDatabase` _asbp_store_vars) (`/Game/111Survival/BuildMode/Grid/WallGridCell.ArrayIndexPoint` _outputvector)) :`WallLevel` _walllevel))
    (:`then_2`
      ;[1 1 1] Determine the right target mesh for animation
      (bind _spawnanimref (`self.SpawnAnimRef`)
        (:`then`
          (switch `int` (`self.WallLevel`)
            (:`1`
              (`SkeletalMeshComponent.PlayAnimation` (`self.mesh_lvl1`) _spawnanimref false))
            (:`2`
              (`SkeletalMeshComponent.PlayAnimation` (`self.mesh_lvl2`) _spawnanimref false))
            (:`3`
              (`SkeletalMeshComponent.PlayAnimation` (`self.mesh_lvl3`) _spawnanimref false))))
        (:`else`)))))

(event `self.TriggerUpgrading`
  ;[1 1 1] Level Up
  ;;[1 1 1] Check conditions
  (bind _asbp_store_vars (cast `/Game/111Survival/BP_StoreVars` (`GameplayStatics.GetGameInstance`)))
  (if (and (`|EnumEquality` (`/Game/111Survival/BP_StoreVars.GameState` _asbp_store_vars) "NewEnumerator4") (not (`KismetSystemLibrary.IsValidClass` (`/Game/111Survival/BP_StoreVars.PlaceableActorType` _asbp_store_vars))))
    ;;[1 1 1] Destroy all other similiar widgets before creating a new one
    (bind _foundwidgets (`WidgetBlueprintLibrary.GetAllWidgetsOfClass` "/Game/111Survival/UI/Upgrades/UI_LevelUp.UI_LevelUp_C"))
    (for _array_element _foundwidgets
      (`/Engine/EditorBlueprintResources/StandardMacros.IsValid` _array_element
        (:`Is Valid`
          (`Widget.RemoveFromParent` _array_element))))
    (bind _asmouse_player_controller (cast `/Game/111Survival/MousePlayerController` (`GameplayStatics.GetPlayerController` 0)))
    (`/Game/111Survival/MousePlayerController.ChangeCameraTarget` _asmouse_player_controller self)
    (bind _menustack (`/Game/111Survival/UI/UI_Frontend.MenuStack` (`/Game/111Survival/MousePlayerController.FrontendRef` _asmouse_player_controller)))
    ;;[1 0 0] Clearing all widgets... ooof
    (`CommonActivatableWidgetContainerBase.ClearWidgets` _menustack)
    (bind _returnvalue (`CommonActivatableWidgetContainerBase.BP_AddWidget` _menustack "/Game/111Survival/UI/Upgrades/UI_LevelUp.UI_LevelUp_C"))
    (bind _output_get (set `self.LevelUpWidget` _returnvalue))
    (set `/Game/111Survival/UI/Upgrades/UI_LevelUp.WallRef` self _output_get)))

(fn `DisableWall`
  (for _array_element (`self.K2_GetComponentsByClass` self "/Script/Engine.SkeletalMeshComponent")
    (`PrimitiveComponent.SetCollisionObjectType` _array_element "ECC_GameTraceChannel2")
    (for (_ _array_index) (`MeshComponent.GetMaterials` _array_element)
      (`PrimitiveComponent.SetMaterial` _array_element _array_index "/Game/111Survival/BuildMode/Materials/BM_PulseMaterial.BM_PulseMaterial")))
  (`ActorComponent.K2_DestroyComponent` (`self.ToughEnemyBlockingNavMesh`)))

(fn `EnableWall`
  (params (WallTransform :type "Transform Structure"))
  (bind _returnvalue (`GameplayStatics.GetActorOfClass` "/Game/111Survival/BuildMode/Grid/WallGridManager.WallGridManager_C"))
  (`/Game/111Survival/BuildMode/Grid/WallGridManager.RebuildWallToCorrectLevel` _returnvalue WallTransform))

(fn `UserConstructionScript`)