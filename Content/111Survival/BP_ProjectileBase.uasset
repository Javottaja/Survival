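; Base projectile Blueprint that damages enemies on overlap, shared by player and turret shots.
; Each collision overlap can destroy it on defense actors, then applies damage to Enemy-tagged BPI_Damageable actors, destroying it unless it pierces.
; A valid owner marks a turret shot, cutting stored Damage to a fifth per hit, so piercing hits compound the reduction.
; An alternative damage-and-destroy function exists but is not called here.
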(event `self.ProjectileCollision.OnComponentBeginOverlap`
  (params (OverlappedComponent :type "PrimitiveComponent Object Reference") (OtherActor :type "Actor Object Reference") (OtherComp :type "PrimitiveComponent Object Reference") (OtherBodyIndex :type Integer) (bFromSweep :type Boolean) (SweepResult :type "HitResult Structure (by ref)"))
  (`self.CheckIfOverlappedDefense` OtherActor)
  (`self.DoDamage` OtherActor))

(fn `CheckIfOverlappedDefense`
  (params (OtherActor :type "Actor Object Reference"))
  (`/Engine/EditorBlueprintResources/StandardMacros.IsValid` OtherActor
    (:`Is Valid`
      (if (`self.IsStoppedByDefenses`)
        (if (`KismetMathLibrary.ClassIsChildOf` (`GameplayStatics.GetObjectClass` OtherActor) "/Game/111Survival/BuildMode/Objects/BP_DefenseBase.BP_DefenseBase_C")
          (`self.K2_DestroyActor`))))))

(fn `DoDamage`
  (params (OtherActor :type "Actor Object Reference"))
  (bind _damage (`self.Damage`))
  (`/Engine/EditorBlueprintResources/StandardMacros.IsValid` OtherActor
    (:`Is Valid`
      ;[1 1 1] Check if target is valid
      (if (and (`KismetSystemLibrary.DoesImplementInterface` OtherActor "/Game/111Survival/BPI_Damageable.BPI_Damageable_C") (`self.ActorHasTag` OtherActor "Enemy"))
        ;[1 1 1] If projectile has an owner (Turret fired it), reduce damage. Otherwise (player fired it), normal damage
        (`/Engine/EditorBlueprintResources/StandardMacros.IsValid` (`self.GetOwner`)
          (:`Is Valid`
            (bind _output_get (set `self.Damage` (* _damage 0.2)))
            (`GameplayStatics.ApplyDamage` OtherActor _output_get))
          (:`Is Not Valid`
            (`GameplayStatics.ApplyDamage` OtherActor _damage)))
        ;[1 1 1] Destroy projectile if it doesn't go through enemies
        (if (not (`self.GoesThroughEnemies`))
          (`self.K2_DestroyActor`))))))

(fn `DoDamageAndDestroyProjectile`
  (params (OtherActor :type "Actor Object Reference"))
  (`/Engine/EditorBlueprintResources/StandardMacros.IsValid` OtherActor
    (:`Is Valid`
      ;[1 1 1] Apply damage on hit
      (if (and (`KismetSystemLibrary.DoesImplementInterface` OtherActor "/Game/111Survival/BPI_Damageable.BPI_Damageable_C") (`self.ActorHasTag` OtherActor "Enemy"))
        (`GameplayStatics.ApplyDamage` OtherActor (`self.Damage`))
        (`self.K2_DestroyActor`)))))

(fn `UserConstructionScript`)