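; BP_EnemyProjectilePulse is an enemy pulse blast whose collision sphere expands from zero toward twice its starting radius over its lifespan.
; On BeginPlay it reads CurrentFPS from the BP_StoreVars game instance and derives a per-frame increment from that rate, capped at 60, and InitialLifeSpan.
; Tick adds that fixed increment without using delta time, so growth depends on the frame rate staying steady.
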(event `self.ReceiveBeginPlay`
  (`self.GetCurrentFPS`)
  (`self.Initialize`))

(event `self.ReceiveTick`
  (params (DeltaSeconds :type "Float (single-precision)"))
  (`self.GrowPulseSize`))

(fn `GetCurrentFPS`
  (bind _asbp_store_vars (cast `/Game/111Survival/BP_StoreVars` (`GameplayStatics.GetGameInstance`)))
  (set `self.CurrentFPS` (`/Game/111Survival/BP_StoreVars.CurrentFPS` _asbp_store_vars)))

(fn `GrowPulseSize`
  (bind _projectilecollision (`self.ProjectileCollision`))
  (`SphereComponent.SetSphereRadius` _projectilecollision (+ (`SphereComponent.SphereRadius` _projectilecollision) (`self.SizeIncrementPerFrame`)) true))

(fn `Initialize`
  ;[1 1 1] Set GrowthModifier
  (set `self.GrowthMultiplier` 2.0)
  ;[1 1 1] Target size of pulse blast
  (set `self.PulseTargetSize` (* (`SphereComponent.SphereRadius` (`self.ProjectileCollision`)) (`self.GrowthMultiplier`)))
  ;[1 1 1] How many frames we have to grow the pulse blast
  (set `self.FrameCount` (* (`KismetMathLibrary.FClamp` (`self.CurrentFPS`) 0.0 60.0) (`self.InitialLifeSpan`)))
  ;[1 1 1] Calculate size increment per frame
  (set `self.SizeIncrementPerFrame` (/ (`self.PulseTargetSize`) (`self.FrameCount`)))
  ;[1 1 1] Initial radius
  (`SphereComponent.SetSphereRadius` (`self.ProjectileCollision`) 0.0 true))

(fn `UserConstructionScript`
  (`parent.UserConstructionScript`))