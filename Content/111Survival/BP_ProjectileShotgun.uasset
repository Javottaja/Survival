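; BP_ProjectileShotgun is a shotgun projectile that grows while in flight and damages actors it overlaps.
; Every Tick multiplies the world scale of both the particle and the collision component by ProjectileSizeIncrement, so visual and hit area expand together.
; The growth compounds per frame without delta-time scaling, so it depends on frame rate.
; Collision begin-overlap passes the other actor to DoDamage, with no filtering in this graph.
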(event `self.ReceiveTick`
  (params (DeltaSeconds :type "Float (single-precision)"))
  (bind _projectilesizeincrement (`self.ProjectileSizeIncrement`))
  ;[1 1 1] Increase the size of projectile while it's flying
  (`SceneComponent.SetWorldScale3D` (`self.ProjectileParticle`) (* (`SceneComponent.K2_GetComponentScale` (`self.ProjectileParticle`)) _projectilesizeincrement))
  (`SceneComponent.SetWorldScale3D` (`self.ProjectileCollision`) (* (`SceneComponent.K2_GetComponentScale` (`self.ProjectileCollision`)) _projectilesizeincrement)))

(event `self.ProjectileCollision.OnComponentBeginOverlap`
  (params (OverlappedComponent :type "PrimitiveComponent Object Reference") (OtherActor :type "Actor Object Reference") (OtherComp :type "PrimitiveComponent Object Reference") (OtherBodyIndex :type Integer) (bFromSweep :type Boolean) (SweepResult :type "HitResult Structure (by ref)"))
  (`self.DoDamage` OtherActor))

(fn `UserConstructionScript`
  (`parent.UserConstructionScript`))